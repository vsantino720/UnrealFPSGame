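; Player character Blueprint with camera-relative movement, look controls and weapon firing.
; On BeginPlay it creates a Reticle widget for the first player and adds it to the viewport.
; Axis inputs move the pawn along the camera manager's forward and right vectors and feed controller yaw and pitch.
; Releasing the left mouse button calls FireWeapon, whose logic is not in these graphs.
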(event `self.ReceiveBeginPlay`
  (bind _returnvalue (`|CreateWidget` "/Game/UI/Reticle.Reticle_C" (`GameplayStatics.GetPlayerController` 0)))
  (`UserWidget.AddToViewport` _returnvalue 0))

(event `Key|LeftMouseButton`
  (params (Key :type "Key Structure"))
  (:`Released`
    (`self.fireWeapon`)))

(event `InputAxis|MoveRight`
  (params (AxisValue :type "Float (single-precision)"))
  ;[1 1 1] Player Movement
  (`self.AddMovementInput` (`self.GetActorRightVector` (`GameplayStatics.GetPlayerCameraManager` 0)) AxisValue))

(event `InputAxis|MoveLeft`
  (params (AxisValue :type "Float (single-precision)"))
  ;[1 1 1] Player Movement
  (`self.AddMovementInput` (`self.GetActorRightVector` (`GameplayStatics.GetPlayerCameraManager` 0)) AxisValue))

(event `InputAxis|MoveForward`
  (params (AxisValue :type "Float (single-precision)"))
  ;[1 1 1] Player Movement
  (`self.AddMovementInput` (`self.GetActorForwardVector` (`GameplayStatics.GetPlayerCameraManager` 0)) AxisValue))

(event `InputAxis|LookHoriz`
  (params (AxisValue :type "Float (single-precision)"))
  (`self.AddControllerYawInput` AxisValue))

(event `InputAxis|LookVertical`
  (params (AxisValue :type "Float (single-precision)"))
  (`self.AddControllerPitchInput` AxisValue))

(fn `UserConstructionScript`)